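; Player-controllable tank Blueprint that wires input to driving, camera orbit and firing.
; BeginPlay hands the barrel and turret to the TankAiming component and both tracks to TankMovement.
; Input drives each track's throttle directly or sends move and rotate intents to TankMovement, while Fire calls TankAiming.
; Aim axes rotate an azimuth gimbal for yaw and the spring arm for pitch separately, scaled by delta time.
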(event `self.ReceiveBeginPlay`
  (`TankAimingComponent.InitializeComponents` (`self.TankAiming`) (`self.Barrel`) (`self.Turret`))
  (`TankMovementComponent.InitializeComponents` (`self.TankMovement`) (`self.LeftTrack`) (`self.RightTrack`)))

(event `InputAction|Fire`
  (params (Key :type "Key Structure" :default "AnyKey"))
  (:`Pressed`
    (`TankAimingComponent.Fire` (`self.TankAiming`))))

(event `InputAxis|Left Track Throttle`
  (params (AxisValue :type "Float (single-precision)"))
  ;[1 1 1] Movement Input Binding
  (`TankTrack.SetThrottle` (`self.LeftTrack`) AxisValue))

(event `InputAxis|AimAzimuth`
  (params (AxisValue :type "Float (single-precision)"))
  ;[1 1 1] Aim Input Binding
  (`SceneComponent.K2_AddLocalRotation` (`self.Azimuth Gimbal`) (`KismetMathLibrary.MakeRotator` 0.0 0.0 (* AxisValue (`GameplayStatics.GetWorldDeltaSeconds`) 100.0)) false false))

(event `InputAxis|Right Track Throttle`
  (params (AxisValue :type "Float (single-precision)"))
  ;[1 1 1] Movement Input Binding
  (`TankTrack.SetThrottle` (`self.RightTrack`) AxisValue))

(event `InputAxis|AimElevation`
  (params (AxisValue :type "Float (single-precision)"))
  ;[1 1 1] Aim Input Binding
  (`SceneComponent.K2_AddLocalRotation` (`self.SpringArm`) (`KismetMathLibrary.MakeRotator` 0.0 (* AxisValue (`GameplayStatics.GetWorldDeltaSeconds`) 100.0)) false false))

(event `InputAxis|MoveForward`
  (params (AxisValue :type "Float (single-precision)"))
  ;[1 1 1] Movement Input Binding
  (`TankMovementComponent.IntendMoveForward` (`self.TankMovement`) AxisValue))

(event `InputAxis|Rotate Right`
  (params (AxisValue :type "Float (single-precision)"))
  ;[1 1 1] Movement Input Binding
  (`TankMovementComponent.IntendRotate` (`self.TankMovement`) AxisValue))

(fn `UserConstructionScript`)